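; BP_CrossHairHUD is a HUD Blueprint that draws wave-completion text on screen; despite its name, it contains no crosshair drawing.
; DrawHUD passes through a gate each frame and draws the text in blue at a position proportional to screen size.
; The WaveCompleted event supplies the text and opens or closes that gate according to the Completed flag on BP_FPSGameModeBase.
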(event `self.ReceiveDrawHUD`
  (params (SizeX :type Integer) (SizeY :type Integer))
  (`/Engine/EditorBlueprintResources/StandardMacros.Gate` true :!label _label
    (:`Exit`
      (`self.DrawText` (stale `WaveCompleted` Text) (struct :`G` 0.205079 :`B` 0.439657 :`A` 1.0) (`KismetMathLibrary.Conv_IntToDouble` (/ SizeX 3)) (`KismetMathLibrary.Conv_IntToDouble` (/ SizeY 8)) "/Game/Fonts/10865_Font.10865_Font"))))

(event `WaveCompleted`
  (params (Text :type String))
  (if (`/Game/Core/BP_FPSGameModeBase.Completed` (cast `/Game/Core/BP_FPSGameModeBase` (`GameplayStatics.GetGameMode`) :!pure true))
    (goto _label :!via `Open`)
    (else
      (goto _label :!via `Close`))))

(fn `UserConstructionScript`)