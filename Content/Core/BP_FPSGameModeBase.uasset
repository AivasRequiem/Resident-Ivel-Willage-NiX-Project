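; FPS game mode that runs escalating waves, spawning a BP_CustomMode actor at the origin on BeginPlay and for each new wave.
; Tick polls Completed, which is not set true here, shows a wave-completed message on BP_CrossHairHUD for three seconds, then halves SpawnFrequency, doubles EnemiesToSpawn and increments WaveNumber.
; SpawnNewWave repeats the logic with a blocking wait on Completed and is not called in this file.
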(event `self.ReceiveBeginPlay`
  (`|SpawnActorFromClass` "/Game/Core/Enemies/BP_CustomMode.BP_CustomMode_C" (`KismetMathLibrary.MakeTransform` (0.0 0.0 0.0)) "Undefined" "OverrideRootScale" null null))

(event `self.ReceiveTick`
  (params (DeltaSeconds :type "Float (single-precision)"))
  (if (`self.Completed`)
    (`/Game/Core/BP_CrossHairHUD.WaveCompleted` (cast `/Game/Core/BP_CrossHairHUD` (`PlayerController.GetHUD` (`GameplayStatics.GetPlayerController` 0)) :!pure true) (`KismetStringLibrary.Concat_StrStr` "Wave " (`KismetStringLibrary.Conv_IntToString` (`self.WaveNumber`)) " completed"))
    (`KismetSystemLibrary.Delay` 3.0)
    (`/Game/Core/BP_CrossHairHUD.WaveCompleted` (cast `/Game/Core/BP_CrossHairHUD` (`PlayerController.GetHUD` (`GameplayStatics.GetPlayerController` 0)) :!pure true) "")
    (set `self.Completed` false)
    (set `self.SpawnFrequency` (* (`self.SpawnFrequency`) 0.5))
    (set `self.EnemiesToSpawn` (* (`self.EnemiesToSpawn`) 2))
    (`/Engine/EditorBlueprintResources/StandardMacros.IncrementInt` (`self.WaveNumber`)
      (:`  `
        (`|SpawnActorFromClass` "/Game/Core/Enemies/BP_CustomMode.BP_CustomMode_C" (`KismetMathLibrary.MakeTransform` (0.0 0.0 0.0)) "Undefined" "OverrideRootScale" null null)))))

(fn `SpawnNewWave`
  (`|SpawnActorFromClass` "/Game/Core/Enemies/BP_CustomMode.BP_CustomMode_C" (`KismetMathLibrary.MakeTransform` (0.0 0.0 0.0)) "Undefined" "OverrideRootScale" null null)
  (while (not (`self.Completed`))
    _)
  (set `self.Completed` false)
  (set `self.SpawnFrequency` (* (`self.SpawnFrequency`) 0.5))
  (set `self.EnemiesToSpawn` (* (`self.EnemiesToSpawn`) 2))
  (`/Engine/EditorBlueprintResources/StandardMacros.IncrementInt` (`self.WaveNumber`)))

(fn `UserConstructionScript`)