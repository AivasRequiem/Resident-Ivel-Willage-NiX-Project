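; Fireball projectile actor that plays a fireball sound on spawn and destroys itself when it overlaps any actor of a different class.
; A fast looping timer billboards its Plane mesh toward the player camera using a look-at rotation with roll and pitch offsets.
; The overlap handler adds a particle system component to the projectile only after calling DestroyActor.
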(event `self.ReceiveBeginPlay`
  (add `self.OnActorBeginOverlap` (delegate `OnOverlap`))
  (`KismetSystemLibrary.K2_SetTimer` null "FaceFireball" 0.01 true)
  (`GameplayStatics.PlaySound2D` "/Game/Sounds/Fireball_SFX.Fireball_SFX" 1.0 1.0 0.0 null null))

(event `OnOverlap` :!signature `self.OnActorBeginOverlap`
  (params (OverlappedActor :type "Actor Object Reference") (OtherActor :type "Actor Object Reference"))
  (`self.OverlapHandler` OtherActor))

(fn `FaceFireball`
  (bind (_returnvalue_roll _returnvalue_pitch _returnvalue_yaw) (`KismetMathLibrary.BreakRotator` (`KismetMathLibrary.Conv_VectorToRotator` (`KismetMathLibrary.Normal` (- (`PlayerCameraManager.GetCameraLocation` (`GameplayStatics.GetPlayerCameraManager` 0)) (`self.K2_GetActorLocation`))))))
  (`SceneComponent.K2_SetWorldRotation` (`self.Plane`) (`KismetMathLibrary.MakeRotator` (+ _returnvalue_roll 180.0) (+ _returnvalue_pitch 90.0) _returnvalue_yaw) false false))

(fn `OverlapHandler`
  (params (OverlapActor :type "Actor Object Reference"))
  (if (not (== (`GameplayStatics.GetObjectClass` OverlapActor) (`GameplayStatics.GetObjectClass` self)))
    (`self.K2_DestroyActor`)
    (`AddComponent|NODE_AddParticleSystemComponent-0`)))

(fn `UserConstructionScript`)