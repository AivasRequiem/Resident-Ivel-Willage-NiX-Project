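; BP_CustomMode is an actor that runs a single enemy wave using the spawn frequency and enemy count from BP_FPSGameModeBase.
; On BeginPlay, a looping timer triggers a random BP_EnemyPortal to spawn until a delay of count times frequency clears it.
; Tick polls for remaining BP_AICharacter actors; once spawning has finished and none remain, it sets the game mode's Completed flag and destroys itself.
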(event `self.ReceiveBeginPlay`
  (bind _asbp_fpsgame_mode_base (cast `/Game/Core/BP_FPSGameModeBase` (`GameplayStatics.GetGameMode`) :!pure true))
  (bind _spawnfrequency (`/Game/Core/BP_FPSGameModeBase.SpawnFrequency` _asbp_fpsgame_mode_base))
  ;[1 1 1] Spawning enemies for one wave
  (`KismetSystemLibrary.K2_SetTimer` null "Spawn Enemy in Random Point" _spawnfrequency true)
  (`KismetSystemLibrary.Delay` (* (`/Game/Core/BP_FPSGameModeBase.EnemiesToSpawn` _asbp_fpsgame_mode_base) _spawnfrequency))
  (`KismetSystemLibrary.K2_ClearTimer` null "Spawn Enemy in Random Point")
  (set `self.AllEnemiesSpawned` true))

(event `self.ReceiveTick`
  (params (DeltaSeconds :type "Float (single-precision)"))
  ;[1 1 1] Check if wave completed
  (bind _outactors (`GameplayStatics.GetAllActorsOfClass` "/Game/Core/Enemies/BP_AICharacter.BP_AICharacter_C"))
  (bind _output_get (set `self.AllEnemiesDead` (== (`KismetArrayLibrary.Array_Length` _outactors) 0)))
  (if (and _output_get (`self.AllEnemiesSpawned`))
    (set `/Game/Core/BP_FPSGameModeBase.Completed` true (cast `/Game/Core/BP_FPSGameModeBase` (`GameplayStatics.GetGameMode`) :!pure true))
    (`self.K2_DestroyActor`)))

(fn `Spawn Enemy in Random Point`
  (bind _outactors (`GameplayStatics.GetAllActorsOfClass` "/Game/Core/Enemies/BP_EnemyPortal.BP_EnemyPortal_C"))
  (`/Game/Core/Enemies/BP_EnemyPortal.Spawn Actor` (`|GetArrayItem` _outactors (`KismetMathLibrary.RandomIntegerInRange` 0 (- (`KismetArrayLibrary.Array_Length` _outactors) 1)))))

(fn `UserConstructionScript`)