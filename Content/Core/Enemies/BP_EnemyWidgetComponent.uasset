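; BP_EnemyWidgetComponent is an enemy's widget component that owns its health, drives its health bar and handles its death.
; It listens to the owner's overlaps, ignores enemy projectiles and subtracts one health per other Projectile hit, pushing the health ratio to BP_EnemyWidget.
; At zero health it plays a death sound, ragdolls the BP_AICharacter, then after a delay spawns an ammo pickup and destroys the owner.
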(event `self.ReceiveBeginPlay`
  (add `Actor.OnActorBeginOverlap` (`self.GetOwner`) (delegate `OnOverlap`))
  (set `self.Health` (`self.MaxHealth`))
  (`self.SetHealth`))

(event `OnOverlap`
  (params (OverlappedActor :type "Actor Object Reference") (OtherActor :type "Actor Object Reference"))
  (bind _returnvalue (`self.GetOwner`))
  (bind _asbp_aicharacter (cast `/Game/Core/Enemies/BP_AICharacter` _returnvalue :!pure true))
  (cast `/Game/Core/BP_EnemyProjectile` OtherActor
    (:`CastFailed`
      (cast `Projectile` OtherActor)
      (bind _output_get (set `self.Health` (- (`self.Health`) 1.0)))
      (if (<= _output_get 0.0)
        ;[1 1 1] Death
        (`GameplayStatics.PlaySoundAtLocation` "/Game/Sounds/SC_Death.SC_Death" (`Actor.K2_GetActorLocation` _returnvalue) (struct) 1.0 1.0 0.0 null null null)
        (set `AI_Character.bIsAlive` false _asbp_aicharacter)
        (`self.SetSimulatePhysics` (`Character.Mesh` _asbp_aicharacter) true)
        (`CharacterMovementComponent.DisableMovement` (`Character.CharacterMovement` _asbp_aicharacter))
        (`KismetSystemLibrary.Delay` 3.0)
        (`|SpawnActorFromClass` "/Game/PickUps/BP_AmmoPickups.BP_AmmoPickups_C" (`Actor.GetTransform` _returnvalue) "Undefined" "OverrideRootScale" null null)
        (`Actor.K2_DestroyActor` _returnvalue)
        (else
          (`self.SetHealth`))))))

(fn `SetHealth`
  (bind _asbp_enemy_widget (cast `/Game/Core/Enemies/BP_EnemyWidget` (`self.GetWidget`)))
  (`/Game/Core/Enemies/BP_EnemyWidget.SetHealthValue` _asbp_enemy_widget (/ (`self.Health`) (`self.MaxHealth`))))